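; BP_PickupCog is a physics-driven puzzle cog that can be picked up and dropped through BP_MotionController.
; Pickup disables mesh physics and attaches the root to the given component in world space; Drop re-enables physics and detaches.
; On mesh hit, it prints correct or incorrect by matching HitComponent's name to "Collision_Cog", testing its own component rather than OtherComp.
; The mating check only prints debug text.
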(event `/Game/VirtualRealityBP/Blueprints/PickupActorInterface.Pickup`
  (params (AttachTo :type "SceneComponent Object Reference"))
  (`PrimitiveComponent.SetSimulatePhysics` (`self.StaticMeshComponent`) false)
  (`SceneComponent.K2_AttachToComponent` (`self.K2_GetRootComponent`) AttachTo "None" "KeepWorld" "KeepWorld" "KeepWorld" false))

(event `/Game/VirtualRealityBP/Blueprints/PickupActorInterface.Drop`
  (`PrimitiveComponent.SetSimulatePhysics` (`self.StaticMeshComponent`) true)
  (`self.K2_DetachFromActor` "KeepWorld" "KeepWorld" "KeepWorld"))

(event `self.StaticMeshComponent.OnComponentHit`
  (params (HitComponent :type "PrimitiveComponent Object Reference") (OtherActor :type "Actor Object Reference") (OtherComp :type "PrimitiveComponent Object Reference") (NormalImpulse :type "Vector Structure") (Hit :type "HitResult Structure (by ref)"))
  (bind _returnvalue (`KismetSystemLibrary.GetDisplayName` HitComponent))
  ;[1 1 1] Check for hit with mating component
  (`|ExecutionSequence`
    (:`then_1`
      (if (`KismetStringLibrary.EqualEqual_StrStr` _returnvalue "Collision_Cog")
        (`KismetSystemLibrary.PrintString` "Correct Block")
        (else
          (`KismetSystemLibrary.PrintString` "Incorrect Block")
          (`KismetSystemLibrary.PrintString` _returnvalue))))))

(fn `UserConstructionScript`)